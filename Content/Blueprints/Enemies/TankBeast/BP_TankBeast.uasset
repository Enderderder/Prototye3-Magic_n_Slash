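; BP_TankBeast is an enemy character with a health bar, driven by the ABP_Jackal animation Blueprint.
; BeginPlay caches the anim instance, binds the health bar widget to itself and sets the AI blackboard's Alive key.
; Damage reduces clamped health, reveals the bar and triggers KillObject at zero; the death event untargets it and clears the animation's Alive flag.
; AI perception originates from a mesh socket; SlamAttack is an empty stub.
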(event `self.ReceiveBeginPlay`
  ;[1 1 1] I hate begin play
  (bind _asabp_jackal (cast `/Game/Blueprints/Enemies/TankBeast/ABP_Jackal` (`SkeletalMeshComponent.GetAnimInstance` (`self.Mesh`)))
    (:`then`
      (set `self.AnimInstance` _asabp_jackal))
    (:`CastFailed`
      _))
  (bind _aswbp_enemy_health_bar (cast `/Game/Blueprints/Widgets/WBP_EnemyHealthBar` (`WidgetComponent.GetUserWidgetObject` (`self.HealthIndicator`))))
  (`/Game/Blueprints/Widgets/WBP_EnemyHealthBar.SetEnemyReference` _aswbp_enemy_health_bar self)
  (`BlackboardComponent.SetValueAsBool` (`AIBlueprintHelperLibrary.GetBlackboard` (`AIBlueprintHelperLibrary.GetAIController` self)) "Alive" true))

(event `self.Receive_EnemyReceiveDamage`
  (params (_value :type "Float (single-precision)") (_bApplyLaunch :type Boolean) (_hitDirection :type "Vector Structure") (_hitPower :type "Float (single-precision)"))
  ;[1 1 1] On receive damage
  (set `self.CurrHealth` (`KismetMathLibrary.FMax` (- (`self.CurrHealth`) _value)))
  (`SceneComponent.SetVisibility` (`self.HealthIndicator`) true false)
  (if (<= (`self.CurrHealth`) 0.0)
    (`self.KillObject`)))

(event `self.Receive_OnObjectKilled`
  ;[1 1 1] On Enemy Killed
  (`self.OnUnTargeted`)
  (set `/Game/Blueprints/Enemies/TankBeast/ABP_Jackal.bAlive` false (`self.AnimInstance`)))

(fn `GetPerceptionLocRot`
  (returns (Location :type "Vector Structure") (Rotation :type "Rotator Structure"))
  (bind (_returnvalue_location _returnvalue_rotation) (`KismetMathLibrary.BreakTransform` (`SceneComponent.GetSocketTransform` (`self.Mesh`) "AIPerceptionSocket" "RTS_World")))
  (return _returnvalue_location _returnvalue_rotation))

(fn `SlamAttack`)

(fn `UserConstructionScript`)
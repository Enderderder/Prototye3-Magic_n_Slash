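; Flame Beast enemy character with a melee hit box and fireballs launched at the blackboard's target location.
; Damage updates the health bar, optionally launches the beast and plays a hurt montage unless stagger-immune, a state randomly gained when staggered.
; Alive and stagger states feed the AI blackboard; death also disables its effects and switches collision to a corpse profile.
; A mesh socket supplies the perception viewpoint.
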(event `self.ReceiveBeginPlay`
  ;[1 1 1] I hate begin play
  (bind _asabp_set_animal (cast `/Game/Blueprints/Enemies/FlameBeast/ABP_SetAnimal` (`SkeletalMeshComponent.GetAnimInstance` (`self.Mesh`))))
  (set `self.AnimInstance` _asabp_set_animal)
  (bind _aswbp_enemy_health_bar (cast `/Game/Blueprints/Widgets/WBP_EnemyHealthBar` (`WidgetComponent.GetUserWidgetObject` (`self.HealthIndicator`))))
  (`/Game/Blueprints/Widgets/WBP_EnemyHealthBar.SetHealth` _aswbp_enemy_health_bar 1.0)
  (`BlackboardComponent.SetValueAsBool` (`AIBlueprintHelperLibrary.GetBlackboard` (`AIBlueprintHelperLibrary.GetAIController` self)) "Alive" true))

(event `self.ReceiveDamage`
  (params (_value :type "Float (single-precision)") (_bApplyLaunch :type Boolean) (_hitDirection :type "Vector Structure") (_hitPower :type "Float (single-precision)"))
  (bind _healthindicator (`self.HealthIndicator`))
  ;[1 1 1] On receive damage
  (set `self.CurrHealth` (`KismetMathLibrary.FMax` (- (`self.CurrHealth`) _value)))
  (`SceneComponent.SetVisibility` _healthindicator true false)
  (bind _aswbp_enemy_health_bar (cast `/Game/Blueprints/Widgets/WBP_EnemyHealthBar` (`WidgetComponent.GetUserWidgetObject` _healthindicator)))
  (`/Game/Blueprints/Widgets/WBP_EnemyHealthBar.SetHealth` _aswbp_enemy_health_bar (/ (`self.CurrHealth`) (`self.MaxHealth`)))
  (if _bApplyLaunch
    (`self.LaunchCharacter` (* _hitDirection _hitPower) true true))
  (if (not (`self.bStaggerImmuned`))
    (`AnimInstance.Montage_Play` (`self.AnimInstance`) "/Game/Assets/Enemies/Set_animal/anim/AM_SetHurt.AM_SetHurt" 1.0 "MontageLength" 0.0 true))
  (if (<= (`self.CurrHealth`) 0.0)
    (`self.KillObject`)))

(event `self.Receive_OnObjectKilled`
  (bind _mesh (`self.Mesh`))
  ;[1 1 1] On Enemy Killed
  (set `self.bAlive` false)
  (`self.OnUnTargeted`)
  (`PrimitiveComponent.SetCollisionProfileName` (`self.CapsuleComponent`) "Corps")
  (`PrimitiveComponent.SetCollisionProfileName` _mesh "Corps")
  (`MeshComponent.SetScalarParameterValueOnMaterials` _mesh "EyeStr" 0.0)
  (`PrimitiveComponent.SetCollisionProfileName` (`self.HitBox`) "Corps")
  (`SceneComponent.SetVisibility` (`self.HealthIndicator`) false false)
  (`ActorComponent.SetActive` (`self.TailFlame`) false false)
  (`BlackboardComponent.SetValueAsBool` (`AIBlueprintHelperLibrary.GetBlackboard` (`AIBlueprintHelperLibrary.GetAIController` self)) "Alive" false)
  (set `/Game/Blueprints/Enemies/FlameBeast/ABP_SetAnimal.bAlive` false (`self.AnimInstance`)))

(event `OnStaggerStart`
  ;[1 1 1] Stagger
  (`BlackboardComponent.SetValueAsBool` (`AIBlueprintHelperLibrary.GetBlackboard` (`AIBlueprintHelperLibrary.GetAIController` self)) "Staggered" true)
  ;;[1 1 1] Have chance to get stagger immune
  (if (`KismetMathLibrary.RandomBool`)
    (set `self.bStaggerImmuned` true)))

(event `OnStaggerEnd`
  ;[1 1 1] Stagger
  (`BlackboardComponent.SetValueAsBool` (`AIBlueprintHelperLibrary.GetBlackboard` (`AIBlueprintHelperLibrary.GetAIController` self)) "Staggered" false))

(event `OnMeleeHitBoxEnable`
  ;[1 1 1] Melee Hit Box
  (`PrimitiveComponent.SetCollisionEnabled` (`self.MeleeHitBox`) "QueryOnly"))

(event `OnMeleeHitBoxDisable`
  ;[1 1 1] Melee Hit Box
  (`PrimitiveComponent.SetCollisionEnabled` (`self.MeleeHitBox`) "NoCollision"))

(event `self.MeleeHitBox.OnComponentBeginOverlap`
  (params (OverlappedComponent :type "PrimitiveComponent Object Reference") (OtherActor :type "Actor Object Reference") (OtherComp :type "PrimitiveComponent Object Reference") (OtherBodyIndex :type Integer) (bFromSweep :type Boolean) (SweepResult :type "HitResult Structure (by ref)"))
  ;[1 1 1] Melee Hit Box
  (bind _asbp_player_character (cast `/Game/Blueprints/Player/BP_PlayerCharacter` OtherActor))
  (`/Game/Blueprints/Player/BP_PlayerCharacter.DamagePlayer` _asbp_player_character 10.0))

(fn `GetPerceptionLocRot`
  (returns (Location :type "Vector Structure") (Rotation :type "Rotator Structure"))
  (bind (_returnvalue_location _returnvalue_rotation) (`KismetMathLibrary.BreakTransform` (`SceneComponent.GetSocketTransform` (`self.Mesh`) "SetAnimalPerceptionSocket" "RTS_World")))
  (return _returnvalue_location _returnvalue_rotation))

(fn `LaunchFireBallAtTarget`
  (`self.LaunchFireBallToLocation` (`BlackboardComponent.GetValueAsVector` (`AIBlueprintHelperLibrary.GetBlackboard` (`self.GetController`)) "TargetLocation")))

(fn `UserConstructionScript`)
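; Boss character that chases the player with AI MoveTo, fights with weapon combos and has a health bar widget.
; A looping timer checks distance to pick random close-range montages or occasional long-range attacks, including a roar unlocked at lower health.
; Attacks set damage and launch force, used by weapon overlaps and a friction-free forward lunge.
; Weapon collision, lunge, facing and fireball spawn are events not called within this graph.
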(event `ERightWep`
  ;[1 1 1] Right Wep Enable/Disable
  (`PrimitiveComponent.SetCollisionEnabled` (`self.RightWep`) "QueryAndPhysics"))

(event `ELeftWep`
  ;[1 1 1] Left Wep Enable/Disable
  (`PrimitiveComponent.SetCollisionEnabled` (`self.LeftWep`) "QueryAndPhysics"))

(event `initialize`
  ;[1 1 1] Initialize Boss
  (set `self.Health` 1000.0)
  (bind _returnvalue (`|CreateWidget` "/Game/Blueprints/Widgets/WBP_BossBar.WBP_BossBar_C"))
  (`UserWidget.AddToViewport` _returnvalue 0)
  (`self.DistancePlayer`)
  (`KismetSystemLibrary.Delay` 0.2)
  (`self.SeekPlayer`))

(event `DLeftWep`
  ;[1 1 1] Left Wep Enable/Disable
  (`PrimitiveComponent.SetCollisionEnabled` (`self.LeftWep`) "NoCollision"))

(event `DRightWep`
  ;[1 1 1] Right Wep Enable/Disable
  (`PrimitiveComponent.SetCollisionEnabled` (`self.RightWep`) "NoCollision"))

(event `self.ReceiveTick`
  (params (DeltaSeconds :type "Float (single-precision)")))

(event `Launcher`
  (bind _charactermovement (`self.CharacterMovement`))
  ;[1 1 1] Launcher
  (set `CharacterMovementComponent.GroundFriction` 0.0 _charactermovement)
  (`self.LaunchCharacter` (+ (* (`self.GetActorForwardVector`) (`self.Launch Force`)) (* (`self.GetActorUpVector`) 1.0)) true)
  (`KismetSystemLibrary.RetriggerableDelay` 0.2)
  (set `CharacterMovementComponent.GroundFriction` 8.0 _charactermovement))

(event `SeekPlayer`
  ;[1 1 1] Seek Player
  (if (`self.IsAttacking`)
    (`MovementComponent.StopMovementImmediately` (`self.CharacterMovement`))
    (else
      (`|AIMoveTo` self (0.0 0.0 0.0) (`GameplayStatics.GetPlayerCharacter` 0) 200.0
        (:`then`
          _)
        (:`OnSuccess`
          _)
        (:`OnFail`
          _))
      (`KismetSystemLibrary.Delay` 0.2)
      (`self.SeekPlayer`))))

(event `DistancePlayer`
  ;[1 1 1] Get PlayerDistance
  (`KismetSystemLibrary.K2_SetTimer` null "PlayerDistance" 1.0 true))

(event `Spell`
  ;[1 1 1] FireBall Spell
  (`|SpawnActorFromClass` "/Game/Blueprints/Spells/Boss_Fireball.Boss_Fireball_C" (`KismetMathLibrary.MakeTransform` (`SceneComponent.K2_GetComponentLocation` (`self.FireZone`)) (`self.K2_GetActorRotation`) (3.0 3.0 3.0)) "Undefined" "OverrideRootScale" null null))

(event `Rotate To Player`
  ;[1 1 1] FacePlayer
  (`self.K2_SetActorRotation` (`KismetMathLibrary.FindLookAtRotation` (`self.K2_GetActorLocation`) (`self.K2_GetActorLocation` (`GameplayStatics.GetPlayerCharacter` 0)))))

(event `CloseRange`
  ;[1 1 1] Boss Combo Moveset
  (set `self.IsAttacking` true)
  (switch `int` (`KismetMathLibrary.RandomIntegerInRange` 0 2)
    (:`0`
      (set `self.AtkMontage` "/Game/Assets/Enemies/Jackal_Boss/anim/jackal_boss_attack_Montage.jackal_boss_attack_Montage")
      (set `self.Launch Force` 350.0)
      (set `self.Damage` 10.0))
    (:`1`
      (set `self.AtkMontage` "/Game/Assets/Enemies/Jackal_Boss/anim/jackal_boss_backhand_Montage.jackal_boss_backhand_Montage")
      (set `self.Launch Force` 350.0)
      (set `self.Damage` 10.0))
    (:`2`
      (set `self.AtkMontage` "/Game/Assets/Enemies/Jackal_Boss/anim/jackal_boss_onetwo_Montage.jackal_boss_onetwo_Montage")
      (set `self.Launch Force` 350.0)
      (set `self.Damage` 15.0)))
  (bind _returnvalue (`self.PlayAnimMontage` (`self.AtkMontage`) :!label _label))
  (`KismetSystemLibrary.Delay` _returnvalue)
  (set `self.IsAttacking` false)
  (`self.SeekPlayer`))

(event `LongRange`
  ;[1 1 1] Boss Combo Moveset
  (set `self.IsAttacking` true)
  (switch `int` (`KismetMathLibrary.RandomIntegerInRange` 0 5)
    (:`0`
      (if (<= (`self.Health`) 750.0)
        (set `self.AtkMontage` "/Game/Assets/Enemies/Jackal_Boss/anim/jackal_boss_roar_Montage.jackal_boss_roar_Montage")
        (goto _label)
        (else
          _)))
    (:`1`
      (set `self.AtkMontage` "/Game/Assets/Enemies/Jackal_Boss/anim/jackal_boss_crossattack_Montage.jackal_boss_crossattack_Montage" :!label _label_2)
      (set `self.Launch Force` 150.0)
      (goto _label))
    (:`2`
      _)
    (:`3`
      (goto _label_2))
    (:`4`
      (goto _label_2))
    (:`5`
      _))
  (set `self.AtkMontage` "/Game/Assets/Enemies/Jackal_Boss/anim/jackal_boss_jump_slash_Montage.jackal_boss_jump_slash_Montage")
  (set `self.Launch Force` 8000.0)
  (set `self.Damage` 30.0)
  (goto _label))

(event `self.LeftWep.OnComponentBeginOverlap`
  (params (OverlappedComponent :type "PrimitiveComponent Object Reference") (OtherActor :type "Actor Object Reference") (OtherComp :type "PrimitiveComponent Object Reference") (OtherBodyIndex :type Integer) (bFromSweep :type Boolean) (SweepResult :type "HitResult Structure (by ref)"))
  ;[1 1 1] Damage Player
  (bind _asbp_player_character (cast `/Game/Blueprints/Player/BP_PlayerCharacter` OtherActor))
  (`/Game/Blueprints/Player/BP_PlayerCharacter.DamagePlayer` _asbp_player_character (`self.Damage`)))

(event `DamageBoss`
  (params (Damage :type "Float (double-precision)"))
  ;[1 1 1] Damage Boss
  (set `self.Health` (- (`self.Health`) Damage)))

(event `self.RightWep.OnComponentBeginOverlap`
  (params (OverlappedComponent :type "PrimitiveComponent Object Reference") (OtherActor :type "Actor Object Reference") (OtherComp :type "PrimitiveComponent Object Reference") (OtherBodyIndex :type Integer) (bFromSweep :type Boolean) (SweepResult :type "HitResult Structure (by ref)"))
  ;[1 1 1] Damage Player
  (bind _asbp_player_character (cast `/Game/Blueprints/Player/BP_PlayerCharacter` OtherActor))
  (`/Game/Blueprints/Player/BP_PlayerCharacter.DamagePlayer` _asbp_player_character (`self.Damage`)))

(fn `PlayerDistance`
  (if (`self.bAlive`)
    (if (not (`self.IsAttacking`))
      (bind _output_get (set `self.Distance` (`KismetMathLibrary.VSize` (- (`self.K2_GetActorLocation`) (`self.K2_GetActorLocation` (`GameplayStatics.GetPlayerCharacter` 0))))))
      (if (>= _output_get 600.0)
        (if (== (`KismetMathLibrary.RandomIntegerInRange` 0 2) 0)
          (`self.LongRange`)
          (else
            (`self.SeekPlayer`)))
        (else
          (`self.CloseRange`))))))

(fn `UserConstructionScript`)
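; BP_BurnableGrassPatch is an actor that scatters a randomized patch of grass when play begins; despite its name, its graphs hold no burning logic.
; BeginPlay clears the instanced mesh component LotsOfGrassComponent, then loops over TotalNumberOfGrasses to add instances.
; Each instance sums two random X/Y offsets, from GeneractionRange and RangeDistribution, and gets random yaw and non-uniform scale, varying most in height.
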(event `self.ReceiveBeginPlay`
  (bind (_returnvalue_roll _returnvalue_pitch _returnvalue_yaw) (`KismetMathLibrary.BreakRotator` (`KismetMathLibrary.RandomRotator` false)))
  (bind _returnvalue (`KismetMathLibrary.RandomFloatInRange` 0.8 1.0))
  (bind _generactionrange (`self.GeneractionRange`))
  (bind _generactionrange_2 (`self.GeneractionRange`))
  (bind _rangedistribution (`self.RangeDistribution`))
  (bind _rangedistribution_2 (`self.RangeDistribution`))
  (`InstancedStaticMeshComponent.ClearInstances` (`self.LotsOfGrassComponent`))
  (for _ (range (+ (`self.TotalNumberOfGrasses`) 1))
    (`InstancedStaticMeshComponent.AddInstance` (`self.LotsOfGrassComponent`) (`KismetMathLibrary.MakeTransform` (`KismetMathLibrary.MakeVector` (+ (`KismetMathLibrary.RandomFloatInRange` (* _generactionrange_2 -1.0) _generactionrange_2) (`KismetMathLibrary.RandomFloatInRange` (* _rangedistribution_2 -1.0) _rangedistribution_2)) (+ (`KismetMathLibrary.RandomFloatInRange` (* _generactionrange -1.0) _generactionrange) (`KismetMathLibrary.RandomFloatInRange` (* _rangedistribution -1.0) _rangedistribution))) (`KismetMathLibrary.MakeRotator` 0.0 0.0 _returnvalue_yaw) (`KismetMathLibrary.MakeVector` _returnvalue _returnvalue (`KismetMathLibrary.RandomFloatInRange` 0.3 1.2))))))

(fn `UserConstructionScript`)
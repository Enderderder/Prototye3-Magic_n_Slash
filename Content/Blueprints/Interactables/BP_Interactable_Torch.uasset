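; Interactable torch that lights when an Ability_Fireball overlaps its fire mesh, which starts hidden.
; Ignite and BlowOutFire toggle the active flag and flame visibility, while Tick calls CheckIsActivated, defined outside this graph.
; It also carries door-style movement: a timeline slides the base mesh to an offset over MoveTime with a camera shake, and reverses to return it.
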(event `self.FireStaticMesh.OnComponentBeginOverlap`
  (params (OverlappedComponent :type "PrimitiveComponent Object Reference") (OtherActor :type "Actor Object Reference") (OtherComp :type "PrimitiveComponent Object Reference") (OtherBodyIndex :type Integer) (bFromSweep :type Boolean) (SweepResult :type "HitResult Structure (by ref)"))
  ;[1 1 1] On Collision with fireball (Ignite)
  (cast `/Game/Blueprints/Spells/Ability_FireBall` OtherActor)
  (`self.Ignite`))

(event `self.ReceiveBeginPlay`
  ;[1 1 1] On BeginPlay
  (`SceneComponent.SetVisibility` (`self.FireStaticMesh`) false false)
  (`self.UpdateTimelinePlayRate`)
  (set `self.Origin` (`self.K2_GetActorLocation`)))

(event `self.ReceiveTick`
  (params (DeltaSeconds :type "Float (single-precision)"))
  ;[1 1 1] Event Tick
  (`self.CheckIsActivated`))

(event `self.Receive_MoveToOffsetPosition`
  ;[1 1 1] Open Door
  (if (not (`self.IsActivated`))
    (`PlayerController.ClientStartCameraShake` :`self` (`GameplayStatics.GetPlayerController` 0) :`Shake` "/Game/Blueprints/Player/DoorShake.DoorShake_C")
    (set `self.IsActivated` true)
    (`self.UpdateTimelinePlayRate`)
    (bind (_direction _newtrack_0) (`Timeline|MoveTimeline` :!label _label)
      (:`Update`
        (`SceneComponent.K2_SetRelativeLocation` (`self.BaseStaticMesh`) (`KismetMathLibrary.VLerp` (0.0 0.0 0.0) (`self.MoveToOffset`) _newtrack_0) false false)))))

(event `self.Recieve_MoveToOriginalPosition`
  ;[1 1 1] Close Door
  (if (`self.IsActivated`)
    (set `self.IsActivated` false)
    (`self.UpdateTimelinePlayRate`)
    (goto _label :!via `Reverse`)))

(event `UpdateTimelinePlayRate`
  ;[1 1 1] Update Timeline PlayRate
  (`TimelineComponent.SetPlayRate` (`self.MoveTimeline`) (/ 1.0 (`self.MoveTime`))))

(fn `BlowOutFire`
  (set `self.InteractableIsActive` false)
  (`SceneComponent.SetVisibility` (`self.FireStaticMesh`) false false))

(fn `Ignite`
  (set `self.InteractableIsActive` true)
  (`SceneComponent.SetVisibility` (`self.FireStaticMesh`) true false))

(fn `UserConstructionScript`)
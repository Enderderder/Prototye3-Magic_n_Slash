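; Interactable pillar that moves between its start transform and an offset, checking its interaction conditions every tick.
; A timeline timed by MoveTime lerps the Cube's relative location and the actor's rotation and scale, playing forward to the offset and reversing back.
; Trigger overlap begin requests the original position and overlap end the offset.
; An optional flag marks movement locked once the forward move finishes.
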(event `self.ReceiveBeginPlay`
  ;[1 1 1] BeginPlay
  (`self.UpdateTimelinePlayRate`)
  (set `self.StartTransform` (`KismetMathLibrary.MakeTransform` (`SceneComponent.RelativeLocation` (`self.Cube`)) (`self.K2_GetActorRotation`) (`self.GetActorScale3D`)))
  (if (not (`self.IsCurrentPosStart`))
    (`self.SetNewMoveTransform` (`self.MoveToOffset`))))

(event `self.ReceiveTick`
  (params (DeltaSeconds :type "Float (single-precision)"))
  ;[1 1 1] Event Tick
  (`self.CheckIsActivated` (`self.InteractionConditions`)))

(event `self.Receive_MoveToOffsetPosition`
  ;[1 1 1] Open/Close Door
  (if (not (`self.IsActivated`))
    (set `self.IsActivated` true)
    (`self.UpdateTimelinePlayRate`)
    (bind (_direction _newtrack_0) (`Timeline|MoveTimeline` :!label _label)
      (:`Update`
        (bind __updatedtransform (`self.LerpMoveTransform` (`self.StartTransform`) _newtrack_0))
        (`self.SetNewMoveTransform` __updatedtransform))
      (:`Finished`
        (if (and (`|EnumEquality` _direction "Forward") (`self.LockOnMoveEnd`))
          (set `self.IsMovementLocked` true))))))

(event `self.Recieve_MoveToOriginalPosition`
  ;[1 1 1] Open/Close Door
  (if (`self.IsActivated`)
    (set `self.IsActivated` false)
    (`self.UpdateTimelinePlayRate`)
    (goto _label :!via `Reverse`)))

(event `UpdateTimelinePlayRate`
  ;[1 1 1] UpdateTimelinePlayRate
  (`TimelineComponent.SetPlayRate` (`self.MoveTimeline`) (/ 1.0 (`self.MoveTime`))))

(event `self.trigger.OnComponentBeginOverlap`
  (params (OverlappedComponent :type "PrimitiveComponent Object Reference") (OtherActor :type "Actor Object Reference") (OtherComp :type "PrimitiveComponent Object Reference") (OtherBodyIndex :type Integer) (bFromSweep :type Boolean) (SweepResult :type "HitResult Structure (by ref)"))
  (`self.Recieve_MoveToOriginalPosition`))

(event `self.trigger.OnComponentEndOverlap`
  (params (OverlappedComponent :type "PrimitiveComponent Object Reference") (OtherActor :type "Actor Object Reference") (OtherComp :type "PrimitiveComponent Object Reference") (OtherBodyIndex :type Integer))
  (`self.Receive_MoveToOffsetPosition`))

(fn `SetNewMovetransform`
  (params (transforms :type "Transform Structure"))
  (`SceneComponent.K2_SetRelativeLocation` (`self.Cube`) (.location transforms) false false)
  (`self.K2_SetActorRotation` (.rotation transforms))
  (`self.SetActorScale3D` (.scale transforms)))

(fn `UserConstructionScript`)
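; Door that opens when every linked interactable in the InteractConditions map has its required activation state, and closes otherwise.
; Tick polls each key's IsActivated against its mapped value, then calls DoorIsOpen or DoorIsClosed.
; Both events act only on a change of IsOpen, toggling the static mesh's visibility and collision instead of animating it.
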(event `self.ReceiveTick`
  (params (DeltaSeconds :type "Float (single-precision)"))
  (bind _interactconditions (`self.InteractConditions`))
  ;[1 1 1] Event Tick
  (bind _keys (`BlueprintMapLibrary.Map_Keys` _interactconditions))
  (set `self.ConditionsMet` true)
  (for (_array_element _array_index) _keys
    (bind _values (`BlueprintMapLibrary.Map_Values` _interactconditions))
    (if (not (== (`InteractableObject.IsActivated` _array_element) (`|GetArrayItem` _values _array_index)))
      (set `self.ConditionsMet` false)))
  (if (`self.ConditionsMet`)
    (`self.DoorIsOpen`)
    (else
      (`self.DoorIsClosed`)))
  (set `self.ConditionsMet` true))

(event `DoorIsOpen`
  (bind _staticmesh (`self.StaticMesh`))
  ;[1 1 1] When Door is Open
  (if (not (`self.IsOpen`))
    (set `self.IsOpen` true)
    (`SceneComponent.SetVisibility` _staticmesh false false)
    (`PrimitiveComponent.SetCollisionEnabled` _staticmesh "NoCollision")))

(event `DoorIsClosed`
  (bind _staticmesh (`self.StaticMesh`))
  ;[1 1 1] When Door is Closed
  (if (`self.IsOpen`)
    (set `self.IsOpen` false)
    (`SceneComponent.SetVisibility` _staticmesh true false)
    (`PrimitiveComponent.SetCollisionEnabled` _staticmesh "QueryAndPhysics")))

(fn `UserConstructionScript`)
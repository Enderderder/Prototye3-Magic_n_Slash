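; Pressure plate interactable that sets its active state when something steps onto its cylinder collider.
; Overlaps respond only to the assigned trigger object, or to any player character when none is assigned.
; Beginning an overlap activates the plate if it is useable, and ending one deactivates it only if the plate is also deactivatable.
; The plate makes itself useable on BeginPlay.
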(event `self.ReceiveBeginPlay`
  (set `self.IsUseable` true))

(event `self.Cylinder.OnComponentBeginOverlap`
  (params (OverlappedComponent :type "PrimitiveComponent Object Reference") (OtherActor :type "Actor Object Reference") (OtherComp :type "PrimitiveComponent Object Reference") (OtherBodyIndex :type Integer) (bFromSweep :type Boolean) (SweepResult :type "HitResult Structure (by ref)"))
  ;[1 1 1] OnPressed
  (`/Engine/EditorBlueprintResources/StandardMacros.IsValid` (`self.ObjectWhichTriggers`)
    (:`Is Valid`
      (if (== OtherActor (`self.ObjectWhichTriggers`))
        (if (`self.IsUseable`) :!label _label
          (set `self.InteractableIsActive` true))))
    (:`Is Not Valid`
      (cast `/Game/Blueprints/Player/BP_PlayerCharacter` OtherActor)
      (goto _label))))

(event `self.Cylinder.OnComponentEndOverlap`
  (params (OverlappedComponent :type "PrimitiveComponent Object Reference") (OtherActor :type "Actor Object Reference") (OtherComp :type "PrimitiveComponent Object Reference") (OtherBodyIndex :type Integer))
  ;[1 1 1] OnExitTrigger
  (`/Engine/EditorBlueprintResources/StandardMacros.IsValid` (`self.ObjectWhichTriggers`)
    (:`Is Valid`
      (if (== OtherActor (`self.ObjectWhichTriggers`))
        (if (and (`self.IsUseable`) (`self.Deactivatable`)) :!label _label_2
          (set `self.InteractableIsActive` false))))
    (:`Is Not Valid`
      (cast `/Game/Blueprints/Player/BP_PlayerCharacter` OtherActor)
      (goto _label_2))))

(fn `UserConstructionScript`)
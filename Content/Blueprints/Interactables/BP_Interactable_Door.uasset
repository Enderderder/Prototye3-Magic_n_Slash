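; Interactable door that moves between its start transform and an offset transform, with a camera shake when it opens.
; Tick polls CheckIsActivated, while open and close events play or reverse the DoorOpen timeline at a rate set by MoveTime.
; Timeline updates feed LerpMoveTransform into SetNewMoveTransform, which applies location to the mesh's relative position but rotation and scale to the actor.
; BeginPlay caches the start transform and can snap to the offset.
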(event `self.ReceiveBeginPlay`
  ;[1 1 1] BeginPlay
  (`self.UpdateTimelinePlayRate`)
  (set `self.StartTransform` (`KismetMathLibrary.MakeTransform` (`SceneComponent.RelativeLocation` (`self.StaticMesh`)) (`self.K2_GetActorRotation`) (`self.GetActorScale3D`)))
  (if (not (`self.IsCurrentPosStart`))
    (`self.SetNewMoveTransform` (`self.MoveToOffset`))))

(event `self.ReceiveTick`
  (params (DeltaSeconds :type "Float (single-precision)"))
  ;[1 1 1] Event Tick
  (`self.CheckIsActivated`))

(event `self.Receive_MoveToOffsetPosition`
  ;[1 1 1] Open Door
  (if (not (`self.IsActivated`))
    (`PlayerController.ClientStartCameraShake` :`self` (`GameplayStatics.GetPlayerController` 0) :`Shake` "/Game/Blueprints/Player/DoorShake.DoorShake_C")
    (set `self.IsActivated` true)
    (`self.UpdateTimelinePlayRate`)
    (bind (_direction _newtrack_0) (`Timeline|DoorOpen` :!label _label)
      (:`Update`
        (bind __updatedtransform (`self.LerpMoveTransform` (`self.StartTransform`) _newtrack_0))
        (`self.SetNewMoveTransform` __updatedtransform)))))

(event `self.Recieve_MoveToOriginalPosition`
  ;[1 1 1] Close Door
  (if (`self.IsActivated`)
    (set `self.IsActivated` false)
    (`self.UpdateTimelinePlayRate`)
    (goto _label :!via `Reverse`)))

(event `UpdateTimelinePlayRate`
  ;[1 1 1] Update Timline PlayRate
  (`TimelineComponent.SetPlayRate` (`self.DoorOpen`) (/ 1.0 (`self.MoveTime`))))

(fn `SetNewMoveTransform`
  (params (Transform :type "Transform Structure"))
  (`SceneComponent.K2_SetRelativeLocation` (`self.StaticMesh`) (.location Transform) false false)
  (`self.K2_SetActorRotation` (.rotation Transform))
  (`self.SetActorScale3D` (.scale Transform)))

(fn `UserConstructionScript`)
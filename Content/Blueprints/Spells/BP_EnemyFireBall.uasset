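; Enemy fireball projectile that damages the player character on contact.
; Each tick it turns to face the velocity of its physics-driven sphere collider and applies a downward acceleration of about twice normal gravity, ignoring mass.
; When the collider overlaps the player character, it deals fixed damage through DamagePlayer and destroys itself; overlaps with other actors are ignored.
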(event `self.ReceiveTick`
  (params (DeltaSeconds :type "Float (single-precision)"))
  (bind _returnvalue (`self.K2_GetActorLocation`))
  (`self.K2_SetActorRotation` (`KismetMathLibrary.FindLookAtRotation` _returnvalue (+ _returnvalue (`SceneComponent.GetComponentVelocity` (`self.SphereCollider`)))))
  (`PrimitiveComponent.AddForce` (`self.SphereCollider`) (`KismetMathLibrary.MakeVector` 0.0 0.0 (* -980.0 2.0)) "None" true))

(event `self.SphereCollider.OnComponentBeginOverlap`
  (params (OverlappedComponent :type "PrimitiveComponent Object Reference") (OtherActor :type "Actor Object Reference") (OtherComp :type "PrimitiveComponent Object Reference") (OtherBodyIndex :type Integer) (bFromSweep :type Boolean) (SweepResult :type "HitResult Structure (by ref)"))
  (bind _asbp_player_character (cast `/Game/Blueprints/Player/BP_PlayerCharacter` OtherActor))
  (`/Game/Blueprints/Player/BP_PlayerCharacter.DamagePlayer` _asbp_player_character 20.0)
  (`self.K2_DestroyActor`))

(fn `UserConstructionScript`)